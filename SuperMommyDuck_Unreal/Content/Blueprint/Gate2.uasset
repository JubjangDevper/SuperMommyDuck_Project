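; Gate actor that opens and closes the Gate2 component in response to a second switch's interaction event.
; On BeginPlay it binds to the Switch2Interacted dispatcher, and each interaction runs a FlipFlop that alternates between the OpenDoor and CloseDoor timelines.
; Each timeline update adds its GatePos track to the gate's current relative location, so movement accumulates per tick rather than interpolating between fixed endpoints.
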(event `OpenGate`
  (bind _gate2 (`self.Gate2`))
  (bind _gate2_2 (`self.Gate2`))
  (`/Engine/EditorBlueprintResources/StandardMacros.FlipFlop`
    (:`A`
      (bind (_direction _gatepos) (`Timeline|OpenDoor`)
        (:`Update`
          (`SceneComponent.K2_SetRelativeLocation` _gate2_2 (+ _gatepos (`SceneComponent.RelativeLocation` _gate2_2)) false false))))
    (:`B`
      (bind (_direction_2 _gatepos_2) (`Timeline|CloseDoor`)
        (:`Update`
          (`SceneComponent.K2_SetRelativeLocation` _gate2 (+ _gatepos_2 (`SceneComponent.RelativeLocation` _gate2)) false false))))))

(event `self.ReceiveBeginPlay`
  (add `/Game/Blueprint/Switch2Interacted.OnSwitch2Interacted` (`self.Switch2InteractedRef`) (delegate `Switch2Interacted`)))

(event `Switch2Interacted`
  (`self.OpenGate`))

(fn `UserConstructionScript`)