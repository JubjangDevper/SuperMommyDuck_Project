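; A rat enemy that wanders the navmesh and ends the game when it overlaps the Duck.
; From BeginPlay it loops AI MoveTo toward random navigable points near itself, pausing briefly after each successful move; a failed move is not retried.
; On overlap with the Duck it shows the GameOver widget and mouse cursor, pauses the game and destroys the Duck.
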(event `self.ReceiveBeginPlay`
  (`self.MoveToRandomLocation`))

(event `MoveToRandomLocation`
  (`|AIMoveTo` self (`NavigationSystemV1.K2_GetRandomLocationInNavigableRadius` (`self.K2_GetActorLocation`) 200.0 null null) null 1.5
    (:`OnSuccess`
      (`KismetSystemLibrary.Delay` 0.5)
      (`self.MoveToRandomLocation`))))

(event `self.ReceiveActorBeginOverlap`
  (params (OtherActor :type "Actor Object Reference"))
  ;[1 1 1] Game Over When Hit
  (bind _asduck (cast `/Game/Blueprint/Duck` OtherActor))
  (bind _returnvalue (`|CreateWidget` "/Game/Widget/GameOver.GameOver_C"))
  (`UserWidget.AddToViewport` _returnvalue 0)
  (set `PlayerController.bShowMouseCursor` true (`GameplayStatics.GetPlayerController` 0))
  (`GameplayStatics.SetGamePaused` true)
  (`self.K2_DestroyActor` _asduck))

(fn `UserConstructionScript`)