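; Boss enemy that hunts the player and ends the game on contact.
; PawnSensing spots a CharacterClass pawn and sends the boss after it with AI MoveTo.
; A Bennyhill 2D track starts on BeginPlay.
; Overlapping the player stops the music, shows the GameOver widget with the mouse cursor, pauses the game and destroys the player character.
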(event `self.PawnSensing.OnSeePawn`
  (params (Pawn :type "Pawn Object Reference"))
  ;[1 1 1] Ai Chasing
  (bind _ascharacter_class (cast `/Game/Blueprint/CharacterClass` Pawn))
  (`|AIMoveTo` self (0.0 0.0 0.0) _ascharacter_class))

(event `self.ReceiveBeginPlay`
  ;[1 1 1] Music
  (bind _returnvalue (`GameplayStatics.SpawnSound2D` "/Game/Music/benny-hill.benny-hill" 1.0 1.0 0.0 null)))

(event `self.ReceiveActorBeginOverlap`
  (params (OtherActor :type "Actor Object Reference"))
  ;[1 1 1] Game Over When Hit
  (bind _ascharacter_class (cast `/Game/Blueprint/CharacterClass` OtherActor))
  (`AudioComponent.Stop` (stale `self.ReceiveBeginPlay` _returnvalue))
  (bind _returnvalue (`|CreateWidget` "/Game/Widget/GameOver.GameOver_C"))
  (`UserWidget.AddToViewport` _returnvalue 0)
  (set `PlayerController.bShowMouseCursor` true (`GameplayStatics.GetPlayerController` 0))
  (`GameplayStatics.SetGamePaused` true)
  (`self.K2_DestroyActor` _ascharacter_class))

(fn `UserConstructionScript`)