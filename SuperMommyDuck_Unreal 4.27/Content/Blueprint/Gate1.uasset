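; Gate actor that alternately opens and closes each time its referenced Switch 1 is interacted with.
; On BeginPlay it binds to the switch's interaction event, which calls OpenGate1, where a FlipFlop picks the OpenDoor or CloseDoor timeline.
; Each timeline update adds its GatePos to Gate1's current relative location, so movement accumulates per tick rather than interpolating between fixed positions.
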(event `OpenGate1`
  (bind _gate1 (`self.Gate1`))
  (bind _gate1_2 (`self.Gate1`))
  (`/Engine/EditorBlueprintResources/StandardMacros.FlipFlop`
    (:`A`
      (bind (_direction _gatepos) (`Timeline|OpenDoor`)
        (:`Update`
          (`SceneComponent.K2_SetRelativeLocation` _gate1_2 (+ (`SceneComponent.RelativeLocation` _gate1_2) _gatepos) false false))))
    (:`B`
      (bind (_direction_2 _gatepos_2) (`Timeline|CloseDoor`)
        (:`Update`
          (`SceneComponent.K2_SetRelativeLocation` _gate1 (+ (`SceneComponent.RelativeLocation` _gate1) _gatepos_2) false false))))))

(event `self.ReceiveBeginPlay`
  (add `/Game/Blueprint/Switch1Interacted.OnSwitch1Interacted` (`self.Switch1InteractedRef`) (delegate `Switch1Interacted`)))

(event `Switch1Interacted`
  (`self.OpenGate1`))

(fn `UserConstructionScript`)