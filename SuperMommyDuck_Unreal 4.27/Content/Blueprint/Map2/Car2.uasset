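; Looping obstacle car for Map2 that ends the game when it hits the player.
; Each tick it moves along its root component's forward vector at Speed, snapping back to StartPos once it travels beyond Distance.
; Overlapping a ThirdPersonCharacter shows the GameOver widget and mouse cursor, pauses the game and destroys the character.
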(event `self.ReceiveTick`
  (params (DeltaSeconds :type "Float (single-precision)"))
  ;[1 1 1] Car Move and Loop
  (`self.K2_AddActorWorldOffset` (* (`SceneComponent.GetForwardVector` (`self.DefaultSceneRoot`)) (* DeltaSeconds (`self.Speed`))))
  (if (> (`KismetMathLibrary.Vector_Distance` (`self.K2_GetActorLocation`) (`self.StartPos`)) (`self.Distance`))
    (`self.K2_SetActorLocation` (`self.StartPos`))))

(event `self.ReceiveActorBeginOverlap`
  (params (OtherActor :type "Actor Object Reference"))
  ;[1 1 1] Game Over When Hit
  (bind _asthird_person_character (cast `/Game/ThirdPersonBP/Blueprints/ThirdPersonCharacter` OtherActor))
  (bind _returnvalue (`|CreateWidget` "/Game/Widget/GameOver.GameOver_C"))
  (`UserWidget.AddToViewport` _returnvalue 0)
  (set `PlayerController.bShowMouseCursor` true (`GameplayStatics.GetPlayerController` 0))
  (`GameplayStatics.SetGamePaused` true)
  (`self.K2_DestroyActor` _asthird_person_character))

(fn `UserConstructionScript`)