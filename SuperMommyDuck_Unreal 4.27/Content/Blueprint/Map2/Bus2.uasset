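; Bus2 is a moving bus obstacle for Map2 that ends the game when it hits the Duck_2 actor.
; Each tick it drives along its root's forward vector at Speed and jumps back to StartPos once it travels beyond Distance, forming an endless loop.
; On overlap with the duck it shows the GameOver_Map2 widget and mouse cursor, pauses the game, destroys the duck and plays a losing sound.
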(event `self.ReceiveTick`
  (params (DeltaSeconds :type "Float (single-precision)"))
  ;[1 1 1] Car Move and Loop
  (`self.K2_AddActorWorldOffset` (* (`SceneComponent.GetForwardVector` (`self.DefaultSceneRoot`)) (* DeltaSeconds (`self.Speed`))))
  (if (> (`KismetMathLibrary.Vector_Distance` (`self.K2_GetActorLocation`) (`self.StartPos`)) (`self.Distance`))
    (`self.K2_SetActorLocation` (`self.StartPos`))))

(event `self.ReceiveActorBeginOverlap`
  (params (OtherActor :type "Actor Object Reference"))
  ;[1 1 1] Game Over When Hit
  (bind _asduck_2 (cast `/Game/Blueprint/Duck_2` OtherActor))
  (bind _returnvalue (`|CreateWidget` "/Game/Widget/GameOver_Map2.GameOver_Map2_C"))
  (`UserWidget.AddToViewport` _returnvalue 0)
  (set `PlayerController.bShowMouseCursor` true (`GameplayStatics.GetPlayerController` 0))
  (`GameplayStatics.SetGamePaused` true)
  (`self.K2_DestroyActor` _asduck_2)
  (`GameplayStatics.SpawnSound2D` "/Game/Music/mixkit-player-losing-or-failing-2042.mixkit-player-losing-or-failing-2042" 1.0 1.0 0.0 null))

(fn `UserConstructionScript`)