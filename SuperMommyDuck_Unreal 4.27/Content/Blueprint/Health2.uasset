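; Health2 is a spinning item pickup that adds one to the SaveAmount count on the Duck_2 actor that touches it.
; On Box overlap it casts to Duck_2, prints a hint to press I to use the item, increments the count, destroys itself and plays a coin sound.
; Tick yaws the actor at a frame-rate-independent speed scaled by its Rotate variable.
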(event `self.Box.OnComponentBeginOverlap`
  (params (OverlappedComponent :type "PrimitiveComponent Object Reference") (OtherActor :type "Actor Object Reference") (OtherComp :type "PrimitiveComponent Object Reference") (OtherBodyIndex :type Integer) (bFromSweep :type Boolean) (SweepResult :type "HitResult Structure (by ref)"))
  (bind _asduck_2 (cast `/Game/Blueprint/Duck_2` OtherActor))
  (if true
    (`KismetSystemLibrary.PrintString` "Get Item. Press I to use.")
    (set `/Game/Blueprint/Duck_2.SaveAmount` (+ (`/Game/Blueprint/Duck_2.SaveAmount` _asduck_2) 1) _asduck_2)
    (`self.K2_DestroyActor`)
    (`GameplayStatics.SpawnSound2D` "/Game/Music/mixkit-game-treasure-coin-2038.mixkit-game-treasure-coin-2038" 1.0 1.0 0.0 null)))

(event `self.ReceiveTick`
  (params (DeltaSeconds :type "Float (single-precision)"))
  (`self.K2_AddActorLocalRotation` (`KismetMathLibrary.MakeRotator` 0.0 0.0 (* (`self.Rotate`) DeltaSeconds 10.0))))

(fn `UserConstructionScript`)