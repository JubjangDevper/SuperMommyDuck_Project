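; Rat enemy Blueprint that wanders between target points and ends the game when it touches the Duck.
; A self-calling event starts on BeginPlay and sends the AI controller toward a random actor from the Target array, repeating after a short random delay.
; Overlapping the Duck shows the GameOver widget and mouse cursor, pauses the game and destroys the Duck.
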(event `self.ReceiveBeginPlay`
  (`self.MoveToRandomLocation`))

(event `MoveToRandomLocation`
  (`AIBlueprintHelperLibrary.SimpleMoveToLocation` (`AIBlueprintHelperLibrary.GetAIController` self) (`self.K2_GetActorLocation` (`KismetArrayLibrary.Array_Random` (`self.Target`))))
  (`KismetSystemLibrary.Delay` (`KismetMathLibrary.RandomFloatInRange` 0.0 2.0))
  (`self.MoveToRandomLocation`))

(event `self.ReceiveActorBeginOverlap`
  (params (OtherActor :type "Actor Object Reference"))
  ;[1 1 1] Game Over When Hit
  (bind _asduck (cast `/Game/Blueprint/Duck` OtherActor))
  (bind _returnvalue (`|CreateWidget` "/Game/Widget/GameOver.GameOver_C"))
  (`UserWidget.AddToViewport` _returnvalue 0)
  (set `PlayerController.bShowMouseCursor` true (`GameplayStatics.GetPlayerController` 0))
  (`GameplayStatics.SetGamePaused` true)
  (`self.K2_DestroyActor` _asduck))

(fn `MoveToRandomLocation`)

(fn `UserConstructionScript`)