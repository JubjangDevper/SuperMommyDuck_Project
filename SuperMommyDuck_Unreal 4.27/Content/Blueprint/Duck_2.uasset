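; Player duck pawn that moves along fixed world axes, jumps with a quack and runs under a three-minute time limit.
; BeginPlay shows the GUI2 widget, then after the delay opens GameOver, pauses, destroys the duck and plays a losing sound.
; Tick drains DuckilngLife at a rate that empties one unit in about that time.
; F opens a paused PauseMenu; 1 saves the level name to an SGO_Player slot.
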(event `Key|F`
  (params (Key :type "Key Structure"))
  (bind _returnvalue (`GameplayStatics.GetPlayerController` 0))
  (bind _pause_menu_reference (`self.Pause Menu Reference`))
  (:`Pressed`
    (`/Engine/EditorBlueprintResources/StandardMacros.IsValid` (`self.Pause Menu Reference`)
      (:`Is Valid`
        (set `PlayerController.bShowMouseCursor` true _returnvalue))
      (:`Is Not Valid`
        (bind _returnvalue_2 (`|CreateWidget` "/Game/Widget/PauseMenu.PauseMenu_C"))
        (set `self.Pause Menu Reference` _returnvalue_2)))
    (`WidgetBlueprintLibrary.SetInputMode_UIOnlyEx` _returnvalue _pause_menu_reference)
    (`UserWidget.AddToViewport` _pause_menu_reference 0)
    (`GameplayStatics.SetGamePaused` true)))

(event `self.ReceiveBeginPlay`
  (bind _returnvalue (`|CreateWidget` "/Game/Widget/GUI2.GUI2_C"))
  (`UserWidget.AddToViewport` _returnvalue 0)
  (`WidgetBlueprintLibrary.SetInputMode_GameOnly` (`GameplayStatics.GetPlayerController` 0))
  (`KismetSystemLibrary.Delay` 180.0)
  (bind _returnvalue_2 (`|CreateWidget` "/Game/Widget/GameOver.GameOver_C"))
  (`UserWidget.AddToViewport` _returnvalue_2 0)
  (set `PlayerController.bShowMouseCursor` true (`GameplayStatics.GetPlayerController` 0))
  (`GameplayStatics.SetGamePaused` true)
  (`self.K2_DestroyActor`)
  (`GameplayStatics.SpawnSound2D` "/Game/Music/mixkit-player-losing-or-failing-2042.mixkit-player-losing-or-failing-2042" 1.0 1.0 0.0 null))

(event `InputAxis|MoveForward`
  (params (AxisValue :type "Float (single-precision)"))
  (`self.AddMovementInput` (0.5 0.0 0.0) AxisValue))

(event `InputAxis|MoveRight`
  (params (AxisValue :type "Float (single-precision)"))
  (`self.AddMovementInput` (0.0 0.5 0.0) AxisValue))

(event `self.ReceiveTick`
  (params (DeltaSeconds :type "Float (single-precision)"))
  (set `self.DuckilngLife` (- (`self.DuckilngLife`) (* DeltaSeconds 0.0056))))

(event `Key|SpaceBar`
  (params (Key :type "Key Structure"))
  (:`Pressed`
    (`self.Jump`)
    (`GameplayStatics.SpawnSound2D` "/Game/Music/Duck_Quack_-_Sound_Effect__HD_.Duck_Quack_-_Sound_Effect__HD_" 1.0 1.0 0.0 null))
  (:`Released`
    (`self.StopJumping`)))

(event `Key|One`
  (params (Key :type "Key Structure"))
  (:`Pressed`
    (bind _returnvalue (`GameplayStatics.DoesSaveGameExist` (`self.Slot Name`)))
    (if _returnvalue
      (bind _returnvalue_2 (`GameplayStatics.LoadGameFromSlot` (`self.Slot Name`)))
      (bind _output_get (set `self.SaverSubClass` _returnvalue_2))
      (bind _assgo_player (cast `/Game/Blueprint/SGO_Player` _output_get))
      (bind _returnvalue_3 (`GameplayStatics.GetCurrentLevelName` true))
      (set `/Game/Blueprint/SGO_Player.LevelName` _returnvalue_3 _assgo_player)
      (else
        (bind _returnvalue_4 (`GameplayStatics.CreateSaveGameObject` "/Game/Blueprint/SGO_Player.SGO_Player_C"))
        (bind _output_get_2 (set `self.SaverSubClass` _returnvalue_4))
        (bind _assgo_player_2 (cast `/Game/Blueprint/SGO_Player` _output_get_2))
        (bind _returnvalue_5 (`GameplayStatics.GetCurrentLevelName` true))
        (set `/Game/Blueprint/SGO_Player.LevelName` _returnvalue_5 _assgo_player_2)))
    (`GameplayStatics.SaveGameToSlot` (`self.SaverSubClass`) (`self.Slot Name`))
    (`KismetSystemLibrary.PrintString` "Saved")))

(fn `NewFunction_0`)

(fn `UserConstructionScript`)